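; Test character Blueprint that tracks a Life value and exercises saving and loading.
; BeginPlay shows Test_Widget and sets Life to full; GetDamage subtracts a fixed amount from it.
; The A and E keys call SaveGame and LoadGame, whose bodies are not in this graph.
; Tick prints a debug message through a Delay, and some unconnected HUD cast and damage nodes remain.
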(event EventBeginPlay
  (bind _returnvalue (UserInterface|CreateWidget "/Game/Compat/HUD/Test_Widget.Test_Widget_C"))
  (UserInterface|Viewport|AddtoViewport _returnvalue 0)
  (Variables|Default|Setlife 1e+02))

(event Collision|EventActorBeginOverlap
  (params (OtherActor :type Actor%20Object%20Reference)))

(event EventTick
  (params (DeltaSeconds :type Float%20%28single-precision%29))
  (Utilities|FlowControl|Delay 3.0)
  (Development|PrintString "Hello"))

(event Input|KeyboardEvents|A
  (params (Key :type Key%20Structure :default "None"))
  (:Pressed
    (Class|CharacterCPP|SaveGame)))

(event Input|KeyboardEvents|E
  (params (Key :type Key%20Structure :default "None"))
  (:Pressed
    (Class|CharacterCPP|LoadGame)))

(fn ConstructionScript)

(fn GetDamage
  (Variables|Default|Setlife (- (Variables|Default|Getlife) 2e+01)))